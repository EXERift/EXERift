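; BP_Floor is a construction-script actor that builds a straight corridor segment of floor, left, right and top pieces from mesh instances, with a set lifespan.
; Four near-identical functions each add instances every 100 units along X, driven by MaxInstances, advancing and then resetting a shared NextPoint.
; The floor pass also records a raised MidPoint, where TBox is placed and scaled relative to the actor's scale.
; The event graph is empty.
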(event `self.ReceiveBeginPlay`)

(event `self.ReceiveActorBeginOverlap`
  (params (OtherActor :type "Actor Object Reference")))

(event `self.ReceiveTick`
  (params (DeltaSeconds :type "Float (single-precision)")))

(fn `Floor`
  (bind _maxinstances (`self.MaxInstances`))
  (bind _returnvalue (`KismetMathLibrary.MakeTransform` (`KismetMathLibrary.MakeVector` (+ (.x (.location (`self.NextPoint`))) 100.0) (.y (.location (`self.NextPoint`))) (.z (.location (`self.NextPoint`)))) (.rotation (`self.NextPoint`)) (.scale (`self.NextPoint`))))
  (for _index (range (+ _maxinstances 1))
    (if (== _index (/ _maxinstances 2))
      (set `self.MidPoint` (`KismetMathLibrary.MakeTransform` (`KismetMathLibrary.MakeVector` (.x (.location (`self.NextPoint`))) (.y (.location (`self.NextPoint`))) (+ (.z (.location (`self.NextPoint`))) 3000.0)) (.rotation (`self.NextPoint`)) (.scale (`self.NextPoint`)))))
    (`InstancedStaticMeshComponent.AddInstance` _returnvalue)
    (set `self.NextPoint` _returnvalue))
  (set `self.NextPoint` (`KismetMathLibrary.MakeTransform` (0.0 0.0 0.0))))

(fn `UserConstructionScript`
  (`self.SetLifeSpan` (`self.InitialLifeSpan`))
  (`InstancedStaticMeshComponent.AddInstance` (`self.InitialTransform`)) ; Creates Initial Mesh
  (`self.Floor`)
  (`self.Wall_Left`)
  (`self.Wall_Right`)
  (`self.Wall_Top`)
  (`SceneComponent.K2_SetRelativeTransform` (`self.TBox`) (`self.MidPoint`) false)
  (`SceneComponent.SetRelativeScale3D` (`self.TBox`) (* (`self.GetActorRelativeScale3D`) (0.1 2.0 300.0))))

(fn `Wall_Left`
  (bind _returnvalue (`KismetMathLibrary.MakeTransform` (`KismetMathLibrary.MakeVector` (+ (.x (.location (`self.NextPoint`))) 100.0) (.y (.location (`self.NextPoint`))) (.z (.location (`self.NextPoint`)))) (.rotation (`self.NextPoint`)) (.scale (`self.NextPoint`))))
  (for _ (range (+ (`self.MaxInstances`) 1))
    (`InstancedStaticMeshComponent.AddInstance` _returnvalue)
    (set `self.NextPoint` _returnvalue))
  (set `self.NextPoint` (`KismetMathLibrary.MakeTransform` (0.0 0.0 0.0))))

(fn `Wall_Right`
  (bind _returnvalue (`KismetMathLibrary.MakeTransform` (`KismetMathLibrary.MakeVector` (+ (.x (.location (`self.NextPoint`))) 100.0) (.y (.location (`self.NextPoint`))) (.z (.location (`self.NextPoint`)))) (.rotation (`self.NextPoint`)) (.scale (`self.NextPoint`))))
  (for _ (range (+ (`self.MaxInstances`) 1))
    (`InstancedStaticMeshComponent.AddInstance` _returnvalue)
    (set `self.NextPoint` _returnvalue))
  (set `self.NextPoint` (`KismetMathLibrary.MakeTransform` (0.0 0.0 0.0))))

(fn `Wall_Top`
  (bind _returnvalue (`KismetMathLibrary.MakeTransform` (`KismetMathLibrary.MakeVector` (+ (.x (.location (`self.NextPoint`))) 100.0) (.y (.location (`self.NextPoint`))) (.z (.location (`self.NextPoint`)))) (.rotation (`self.NextPoint`)) (.scale (`self.NextPoint`))))
  (for _ (range (+ (`self.MaxInstances`) 1))
    (`InstancedStaticMeshComponent.AddInstance` _returnvalue)
    (set `self.NextPoint` _returnvalue))
  (set `self.NextPoint` (`KismetMathLibrary.MakeTransform` (0.0 0.0 0.0))))