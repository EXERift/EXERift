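; Spawner actor that places obstacles and power-ups at random points inside its Box bounds while the OculusCharacter player is alive.
; Tick runs through a latent Delay to pace spawns, then a percentage roll picks an obstacle or one of two power-ups.
; A dead player or non-positive delay triggers a SetActive(false) call.
; The construction script intends to match projectile velocity to character speed, but its cast has no input.
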(event `self.ReceiveTick`
  (params (DeltaSeconds :type "Float (single-precision)"))
  (set `self.StreamSeed` (`KismetMathLibrary.FFloor` (`KismetSystemLibrary.GetGameTimeInSeconds`)))
  (bind _asoculus_character (cast `/Game/Blueprints/OculusCharacter` (`GameplayStatics.GetPlayerPawn` 0))) ; REPLACE WITH HIGHSCORE MENU
  (if (and (== (`/Game/Blueprints/OculusCharacter.Dead` _asoculus_character) false) (> (`self.spawndelay`) 0.0))
    (`KismetSystemLibrary.Delay` (`self.SpawnDelay`))
    (if (<= (`KismetMathLibrary.RandomIntegerInRange` 1 100) (`self.powerupchance`))
      (switch `int` (`KismetMathLibrary.RandomIntegerInRange` 0 1)
        (:`Default`
          (`KismetSystemLibrary.PrintString` "PowerUp Index Out Of Range"))
        (:`0`
          (bind _worldlocation (`self.GetRandomSpawnPoint`))
          (`|SpawnActorFromClass` "/Game/Blueprints/Actors/PowerUp1.PowerUp1_C" (`KismetMathLibrary.Conv_VectorToTransform` _worldlocation)))
        (:`1`
          (bind _worldlocation_2 (`self.GetRandomSpawnPoint`))
          (`|SpawnActorFromClass` "/Game/Blueprints/Actors/PowerUp2.PowerUp2_C" (`KismetMathLibrary.Conv_VectorToTransform` _worldlocation_2))))
      (else
        (bind _worldlocation_3 (`self.GetRandomSpawnPoint`))
        (`|SpawnActorFromClass` "/Game/Blueprints/Actors/Obstacle1_BP.Obstacle1_BP_C" (`KismetMathLibrary.MakeTransform` _worldlocation_3))))
    (else
      (`ActorComponent.SetActive` false))))

(fn `GetRandomSpawnPoint`
  (returns (Worldlocation :type "Object.Vector Structure"))
  (bind (_origin _boxextent) (`KismetSystemLibrary.GetComponentBounds` (`self.Box`)))
  (bind (_returnvalue_x _returnvalue_y _returnvalue_z) (`KismetMathLibrary.BreakVector` (- _origin _boxextent)))
  (bind (_returnvalue_x_2 _returnvalue_y_2 _returnvalue_z_2) (`KismetMathLibrary.BreakVector` (+ _origin _boxextent)))
  (return (`KismetMathLibrary.MakeVector` (`KismetMathLibrary.RandomFloatInRange` _returnvalue_x _returnvalue_x_2) (`KismetMathLibrary.RandomFloatInRange` _returnvalue_y _returnvalue_y_2) (`KismetMathLibrary.RandomFloatInRange` _returnvalue_z _returnvalue_z_2))))

(fn `UserConstructionScript`
  (bind _asoculus_character (cast `/Game/Blueprints/OculusCharacter` null))
  (`ProjectileMovementComponent.SetVelocityInLocalSpace` (`self.ProjectileMovement`) (`KismetMathLibrary.MakeVector` 1.0 (* (`/Game/Blueprints/OculusCharacter.Forward` _asoculus_character) (`/Game/Blueprints/OculusCharacter.MoveSpeed` _asoculus_character)) 1.0)))