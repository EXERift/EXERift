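; PowerUp3 is an actor Blueprint, apparently a power-up pickup that moves through the level via a ProjectileMovement component.
; Its Construction Script does all the setup: a Speed variable drives both initial and max projectile speed, gravity is disabled and a lifespan is set.
; It also fixes the actor's rotation and applies a uniform scale from NewScale.
; The Event Graph holds only disabled placeholder events, so no overlap or pickup logic lives here.
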(event `self.ReceiveBeginPlay`)

(event `self.ReceiveActorBeginOverlap`
  (params (OtherActor :type "Actor Object Reference")))

(event `self.ReceiveTick`
  (params (DeltaSeconds :type "Float (single-precision)")))

(fn `UserConstructionScript`
  (bind _projectilemovement (`self.ProjectileMovement`))
  (bind _newscale (`self.NewScale`))
  (bind _output_get (set `ProjectileMovementComponent.InitialSpeed` (`self.Speed`) _projectilemovement))
  (set `ProjectileMovementComponent.MaxSpeed` _output_get _projectilemovement)
  (`PrimitiveComponent.SetEnableGravity` false)
  (`self.SetLifeSpan` (`self.InitialLifeSpan`))
  (`self.SetActorRotation` (`KismetMathLibrary.MakeRot` 90.0 90.0))
  (`self.SetActorRelativeScale3D` (`KismetMathLibrary.MakeVector` _newscale _newscale _newscale)))