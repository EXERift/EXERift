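; Obstacle1_BP is an obstacle actor whose construction script configures its motion and randomizes its appearance.
; It sets the projectile movement's initial and max speed from Speed, disables gravity and adds a random positive X linear velocity to its physics body.
; It applies a uniform scale from NewScale and a random pitch with fixed yaw and roll, then randomly swaps the mesh to a triangular pyramid.
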(fn `UserConstructionScript`
  (bind _projectilemovement1 (`self.ProjectileMovement1`))
  (bind _newscale (`self.NewScale`))
  (bind _output_get (set `ProjectileMovementComponent.InitialSpeed` (`self.Speed`) _projectilemovement1))
  (set `ProjectileMovementComponent.MaxSpeed` _output_get _projectilemovement1)
  (`PrimitiveComponent.SetEnableGravity` false) ; Turn off Gravity
  ;[1 1 1] Velocity Setup
  (`PrimitiveComponent.SetPhysicsLinearVelocity` (`KismetMathLibrary.MakeVector` (* (`KismetMathLibrary.RandomFloat`) 5000.0)) true)
  (`self.SetActorRelativeScale3D` (`KismetMathLibrary.MakeVector` _newscale _newscale _newscale))
  (`self.SetActorRotation` (`KismetMathLibrary.MakeRot` (* (`KismetMathLibrary.RandomFloat`) 100.0) 90.0 90.0))
  (if (`KismetMathLibrary.RandomBool`)
    (`StaticMeshComponent.SetStaticMesh` "/Game/StarterContent/Shapes/Shape_TriPyramid.Shape_TriPyramid")))