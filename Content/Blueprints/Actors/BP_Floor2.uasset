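; BP_Floor2 is a self-extending floor segment that spawns another BP_Floor2 when an actor tagged Player overlaps it.
; The construction script sets the segment's lifespan, then SpawnMultiples lays rotated instances along X while recording a midpoint and an end point.
; The trigger box moves to the midpoint and scales from the instance scale.
; The computed end point, raised by a large Z offset, serves directly as the next segment's spawn transform.
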(event `self.ReceiveBeginPlay`)

(event `self.ReceiveActorBeginOverlap`
  (params (OtherActor :type "Actor Object Reference"))
  (if (`self.ActorHasTag` OtherActor "Player")
    (`|SpawnActorFromClass` "BP_Floor2_C" (`self.EndPoint`) true)))

(event `self.ReceiveTick`
  (params (DeltaSeconds :type "Float (single-precision)")))

(fn `SpawnMultiples`
  (returns (NewScale :type "Object.Vector Structure") (EndPoint :type "Object.Transform Structure"))
  (bind _newscale_x (`KismetMathLibrary.BreakVector` (`self.NewScale`)))
  (bind _maxinstances (`self.MaxInstances`))
  (bind _returnvalue (`KismetMathLibrary.MakeTransform` (`KismetMathLibrary.MakeVector` (+ (.x (.location (`self.NextPoint`))) (`self.Offset`)) (.y (.location (`self.NextPoint`))) (.z (.location (`self.NextPoint`)))) (struct :`Pitch` 90.0) (`self.NewScale`)))
  (for _index (range (+ _maxinstances 1))
    (set `self.TotalLength` (+ _newscale_x (`self.TotalLength`)))
    (if (== _index (/ _maxinstances 2))
      (set `self.MidPoint` (`KismetMathLibrary.MakeTransform` (.location (`self.NextPoint`)) (struct :`Pitch` 90.0) (`self.NewScale`)))
      (elif (== _index (- _maxinstances 1))
        (bind _output_get (set `self.EndPoint` (`KismetMathLibrary.MakeTransform` (`KismetMathLibrary.MakeVector` (+ (`self.TotalLength`) (.x (.location (`self.NextPoint`)))) (.y (.location (`self.NextPoint`))) (+ (.z (.location (`self.NextPoint`))) 50000.0)) (struct) (1.0 1.0 1.0))))
        (return (`self.NewScale`) _output_get)
        (else
          _)))
    (`InstancedStaticMeshComponent.AddInstance` _returnvalue)
    (set `self.NextPoint` _returnvalue))
  (set `self.NextPoint` (`KismetMathLibrary.MakeTransform` (0.0 0.0 0.0))))

(fn `UserConstructionScript`
  (`self.SetLifeSpan` (`self.InitialLifeSpan`))
  (bind (_newscale _endpoint) (`self.SpawnMultiples`))
  (set `self.EndPoint` _endpoint)
  (`SceneComponent.K2_SetRelativeTransform` (`self.Box`) (`self.MidPoint`) false)
  (`SceneComponent.SetRelativeScale3D` (`self.Box`) (* _newscale (3.5 3.5 1.0))))