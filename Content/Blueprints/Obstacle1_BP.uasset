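; Obstacle1_BP is a moving obstacle that destroys itself when it overlaps an actor tagged EndBox.
; Its construction script applies Speed to the projectile movement as both initial and maximum speed, disables gravity and randomizes rotation.
; It also picks one of three glowy materials, adding a matching actor tag, and randomly swaps the mesh to a triangular pyramid at unit scale.
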(event `self.ReceiveActorBeginOverlap`
  (params (OtherActor :type "Actor Object Reference"))
  (if (`self.ActorHasTag` OtherActor "EndBox")
    (`self.K2_DestroyActor`)))

(fn `UserConstructionScript`
  (bind _tags (`self.Tags`))
  (bind _projectilemovement1 (`self.ProjectileMovement1`))
  (bind _output_get (set `ProjectileMovementComponent.InitialSpeed` (`self.Speed`) _projectilemovement1))
  (set `ProjectileMovementComponent.MaxSpeed` _output_get _projectilemovement1)
  (`PrimitiveComponent.SetEnableGravity` false)
  (`self.SetActorRotation` (`KismetMathLibrary.RandomRotator` false))
  (switch `int` (`KismetMathLibrary.RandomInteger` 3)
    (:`Default`
      (`PrimitiveComponent.SetMaterial` 0 "/Game/Custom/Glowy.Glowy" :!label _label)
      (`KismetArrayLibrary.Array_Add` _tags "Glowy"))
    (:`0`
      (goto _label))
    (:`1`
      (`PrimitiveComponent.SetMaterial` 0 "/Game/Custom/Glowy2.Glowy2")
      (`KismetArrayLibrary.Array_Add` _tags "Glowy2"))
    (:`2`
      (`PrimitiveComponent.SetMaterial` 0 "/Game/Custom/Glowy3.Glowy3")
      (`KismetArrayLibrary.Array_Add` _tags "Glowy3")))
  (`self.SetActorScale3D` (`KismetMathLibrary.MakeVector` 1.0 1.0 1.0))
  (if (`KismetMathLibrary.RandomBool`)
    (`StaticMeshComponent.SetStaticMesh` "/Game/StarterContent/Shapes/Shape_TriPyramid.Shape_TriPyramid")
    (`self.SetActorScale3D` (`KismetMathLibrary.MakeVector` 1.0 1.0 1.0))))